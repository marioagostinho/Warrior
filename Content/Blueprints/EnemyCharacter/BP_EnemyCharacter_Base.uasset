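; Base enemy character Blueprint that handles death with a dissolve effect.
; On death it pauses the mesh animation, disables capsule collision and async-loads the given Niagara system.
; That system spawns attached to the mesh, tinted by the material's DissolveEdgeColor.
; A timeline scaled to TotalDissolveTime drives DissolveAmount on body and equipped weapon, then destroys both actors.
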(event `/Game/Blueprints/EnemyCharacter/BPI_EnemyDeath.OnEnemyDied`
  (params (DissolveNiagaraSystem :type "NiagaraSystem Soft Object Reference"))
  (bind _returnvalue (`PawnCombatComponent.GetCharacterCurrentEquipped` (`self.EnemyCombatComponent`)))
  (bind _returnvalue_2 (`PawnCombatComponent.GetCharacterCurrentEquipped` (`self.EnemyCombatComponent`)))
  (`|ExecutionSequence`
    (:`then_0`
      (set `SkeletalMeshComponent.bPauseAnims` true (`self.Mesh`))
      (`PrimitiveComponent.SetCollisionEnabled` (`self.CapsuleComponent`) "NoCollision"))
    (:`then_1`
      (bind _object (`|LoadAsset` DissolveNiagaraSystem)
        (:`Completed`
          (`self.TriggerNiagaraSystem` _object)
          (`TimelineComponent.SetPlayRate` (`self.DissolveTimeline`) (/ 1.0 (`self.TotalDissolveTime`)))
          (bind (_direction _normalizefloattrack) (`Timeline|DissolveTimeline` :!via `PlayFromStart`)
            (:`Update`
              (`MeshComponent.SetScalarParameterValueOnMaterials` (`self.Mesh`) "DissolveAmount" _normalizefloattrack)
              (`/Engine/EditorBlueprintResources/StandardMacros.IsValid` _returnvalue_2
                (:`Is Valid`
                  (`MeshComponent.SetScalarParameterValueOnMaterials` (`WarriorWeaponBase.WeaponMesh` _returnvalue_2) "DissolveAmount" _normalizefloattrack))))
            (:`Finished`
              (`/Engine/EditorBlueprintResources/StandardMacros.IsValid` _returnvalue
                (:`Is Valid`
                  (`self.K2_DestroyActor` _returnvalue))
                (:`Is Not Valid`
                  _))
              (`self.K2_DestroyActor`))))))))

(fn `TriggerNiagaraSystem`
  (params (NiagaraSystem :type "Object Object Reference"))
  (bind _mesh (`self.Mesh`))
  (bind _asniagara_system (cast `NiagaraSystem` NiagaraSystem))
  (bind _returnvalue (`NiagaraFunctionLibrary.SpawnSystemAttached` _asniagara_system (`self.Mesh`) "None" (0.0 0.0 0.0) (struct) "KeepRelativeOffset" true))
  (bind _returnvalue_2 (`PrimitiveComponent.CreateDynamicMaterialInstance` _mesh 0 (`PrimitiveComponent.GetMaterial` _mesh 0) "None"))
  (bind _returnvalue_3 (`MaterialInstanceDynamic.K2_GetVectorParameterValue` _returnvalue_2 "DissolveEdgeColor"))
  (`NiagaraComponent.SetNiagaraVariableLinearColor` _returnvalue "DissolveParticleColor" _returnvalue_3))

(fn `UserConstructionScript`)